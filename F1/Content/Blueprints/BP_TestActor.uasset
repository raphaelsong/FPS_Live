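; BP_TestActor is a test actor that prints debug strings for an array loop and a simple function call.
; On BeginPlay it loops over the Numbers array and prints each index and element through Format Text.
; Every Tick it calls TestFunc, which adds two inputs, with constant arguments and prints the sum.
; The overlap event and construction script are empty.
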(event EventBeginPlay
  (for (_array_element _array_index) (Variables|Default|GetNumbers)
    (Development|PrintString (Utilities|String|ToString(Text) (Utilities|Text|FormatText "{Index} : {Element}" _array_index _array_element)))))

(event Collision|EventActorBeginOverlap
  (params (OtherActor :type Actor%20Object%20Reference)))

(event EventTick
  (params (DeltaSeconds :type Float%20%28single-precision%29))
  (bind _result (CallFunction|TestFunc 10 20))
  (Development|PrintString (Utilities|String|ToString(Integer) _result)))

(fn ConstructionScript)

(fn TestFunc
  (params (A :type Integer) (B :type Integer))
  (bind _output_get (LocalVariables|SetTemp (+ A B)))
  (return _output_get))